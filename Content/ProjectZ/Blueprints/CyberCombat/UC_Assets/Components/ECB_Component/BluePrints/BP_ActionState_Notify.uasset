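; Animation notify state that puts the owner's AC_HitReaction component into a chosen action state for a span of an animation.
; On begin it sets that state and applies the configured movement mode and collision response through the component.
; On end it restores Walking and Block, and resets the action state to the first enum entry only if nothing else changed it.
; The notify's display name comes from the selected action state.
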(fn ReceivedNotifyBegin
  (params (MeshComp :type Skeletal%20Mesh%20Component%20Object%20Reference) (Animation :type Anim%20Sequence%20Base%20Object%20Reference) (TotalDuration :type Float%20%28single-precision%29) (EventReference :type Anim%20Notify%20Event%20Reference%20Structure%20%28by%20ref%29))
  (bind _returnvalue (Components|GetOwner MeshComp))
  (bind _returnvalue_2 (Actor|GetComponentbyClass _returnvalue "/Game/ProjectZ/Blueprints/CyberCombat/UC_Assets/Components/HitReactionComponent/BluePrint/AC_HitReaction.AC_HitReaction_C"))
  (Utilities|IsValid _returnvalue_2
    (:Is%20Valid
      (Default|SetActionState _returnvalue_2 (Variables|Default|GetActionState))
      (Default|SetMovement/Collision _returnvalue_2 (Variables|Default|GetNew%20Movement%20Mode) (Variables|Default|GetNew%20Collision%20Response))
      (return true))
    (:Is%20Not%20Valid
      (return true))))

(fn ReceivedNotifyEnd
  (params (MeshComp :type Skeletal%20Mesh%20Component%20Object%20Reference) (Animation :type Anim%20Sequence%20Base%20Object%20Reference) (EventReference :type Anim%20Notify%20Event%20Reference%20Structure%20%28by%20ref%29))
  (bind _returnvalue (Components|GetOwner MeshComp))
  (bind _returnvalue_2 (Actor|GetComponentbyClass _returnvalue "/Game/ProjectZ/Blueprints/CyberCombat/UC_Assets/Components/HitReactionComponent/BluePrint/AC_HitReaction.AC_HitReaction_C"))
  (Utilities|IsValid _returnvalue_2
    (:Is%20Valid
      (Default|SetMovement/Collision _returnvalue_2 "MOVE_Walking" "ECR_Block")
      (if (== (Default|GetActionState _returnvalue_2) (Variables|Default|GetActionState))
        (Default|SetActionState _returnvalue_2 "NewEnumerator0")
        (return true)))
    (:Is%20Not%20Valid
      (return false))))

(fn GetNotifyName
  (return (Utilities|String|EnumtoString (Variables|Default|GetActionState))))