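; BP_Weapon is a data-driven weapon actor that sets up its own mesh and, for dual weapons, an off-hand companion.
; The construction script looks up the stored weapon name in DT_WeaponState and caches the row as WeaponData.
; BeginPlay applies that row's static mesh and, if flagged dual, spawns a BP_2ndWeapon snapped to the second holster socket on the owner's skeletal mesh.
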(event EventBeginPlay
  (bind _weapondata (Variables|Default|GetWeaponData))
  (bind _weaponsetup (Utilities|Struct|BreakF_WeaponState _weapondata))
  (bind (_weaponmesh _dualweapons _2ndweapon) (Utilities|Struct|BreakF_WeaponSetup _weaponsetup))
  (Components|StaticMesh|SetStaticMesh (Variables|Default|GetWeaponMesh) _weaponmesh)
  (if _dualweapons
    (bind _returnvalue (Game|SpawnActorfromClass "/Game/ProjectZ/Blueprints/CyberCombat/UC_Assets/Components/ECB_Component/BluePrints/BP_2ndWeapon.BP_2ndWeapon_C" (Math|Transform|MakeTransform "0, 0, 0" "0, 0, 0" "1.000000,1.000000,1.000000") "Undefined" "OverrideRootScale" (Components|GetOwner) _2ndweapon 0))
    (Variables|Default|Set2ndWeapon _returnvalue)
    (Transformation|AttachComponentToComponent (Variables|Default|Get2ndWeapon) (Actor|GetComponentbyClass (Components|GetOwner) "/Script/Engine.SkeletalMeshComponent") (Utilities|Struct|BreakF_WeaponSetup (Utilities|Struct|BreakF_WeaponState (Variables|Default|GetWeaponData))) "SnapToTarget" "SnapToTarget" "KeepRelative" true)))

(event Collision|EventActorBeginOverlap
  (params (OtherActor :type Actor%20Object%20Reference)))

(event EventTick
  (params (DeltaSeconds :type Float%20%28single-precision%29)))

(fn ConstructionScript
  (bind _returnvalue (Utilities|GetDataTableRow "/Game/ProjectZ/Blueprints/CyberCombat/UC_Assets/Components/ECB_Component/DataTables/DT_WeaponState.DT_WeaponState" (Utilities|Struct|BreakF_StoredWeapons (Variables|Default|GetStoredWeapon)))
    (:then
      (Variables|Default|SetWeaponData _returnvalue))))