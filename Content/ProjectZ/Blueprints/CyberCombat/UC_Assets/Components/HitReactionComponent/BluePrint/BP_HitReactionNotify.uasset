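; BP_HitReactionNotify is an animation notify, shown as "Hit Reaction", that carries the hit settings for a combat animation.
; When it fires, it finds the mesh owner's AC_HitReaction component and, if valid, passes those settings through SetHitReactionMessage.
; The settings cover damage and strength, directional, air and blocked reactions, sound and particle effects, plus camera shake, decal and push-back from a HitFeedback struct.
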(fn ReceivedNotify
  (params (MeshComp :type Skeletal%20Mesh%20Component%20Object%20Reference) (Animation :type Anim%20Sequence%20Base%20Object%20Reference) (EventReference :type Anim%20Notify%20Event%20Reference%20Structure%20%28by%20ref%29))
  (bind _returnvalue (Components|GetOwner MeshComp))
  (bind _hit_feedback (Variables|Default|GetHit%20Feedback))
  (bind (_camerashake _shakesale _usehitdecal _hitdecal _usehitfeedback) (Utilities|Struct|BreakF_HitFeedBack _hit_feedback))
  (bind _returnvalue_2 (Actor|GetComponentbyClass _returnvalue "/Game/ProjectZ/Blueprints/CyberCombat/UC_Assets/Components/HitReactionComponent/BluePrint/AC_HitReaction.AC_HitReaction_C"))
  (Utilities|IsValid _returnvalue_2
    (:Is%20Valid
      (Class|BIReactionInterface|SetHitReaction(Message) _returnvalue_2 (Variables|Default|GetIs%20Air%20Launch%20Attack) (Variables|Default|GetHit%20Strength) (Variables|Default|GetDamage) (Variables|Default|GetFront%20Hit%20Reaction) (Variables|Default|GetBack%20Hit%20Reaction) (Variables|Default|GetAir%20Hit%20Reaction) (Variables|Default|GetCan%20be%20Blocked?) (Variables|Default|GetBlock%20Reaction) (Variables|Default|GetUse%20Blocked%20Reaction%20Anim?) (Variables|Default|GetBlocked%20Reaction%20Anim) (Variables|Default|GetHit%20Sound%20FX) (Variables|Default|GetHit%20Particle%20FX) _camerashake _shakesale _usehitdecal _hitdecal _usehitfeedback)
      (return false))))

(fn GetNotifyName
  (return "Hit Reaction"))